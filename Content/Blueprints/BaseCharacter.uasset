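; Base character for NagaQuest that holds RPG vitals, experience and level, and adds a StatsUI widget to the viewport.
; On BeginPlay it builds an enum-indexed Vitals array, then overwrites stats from the save slot named after the game mode when a game was loaded.
; LevelUp grows the next-level XP requirement on a tiered, tapering curve, scaling and refilling vitals by LevelMod only in the top tier.
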(event `self.ReceiveBeginPlay`
  (`self.SetupVitals`)
  (`self.LoadStats`)
  (`self.SetupHud`))

(event `self.ReceiveActorBeginOverlap`
  (params (OtherActor :type "Actor Object Reference")))

(event `self.ReceiveTick`
  (params (DeltaSeconds :type "Float (single-precision)")))

(fn `LevelUp`
  (bind _level (`self.Level`))
  (bind _nextlevelexp (`self.NextLevelExp`))
  (bind _vitals (`self.Vitals`))
  (set `self.Level` (+ _level 1))
  (if (< _level 40)
    (set `self.NextLevelExp` (`KismetMathLibrary.FTrunc` (* _nextlevelexp 1.4)))
    (elif (< _level 80)
      (set `self.NextLevelExp` (`KismetMathLibrary.FTrunc` (* _nextlevelexp 1.2)))
      (else
        (set `self.NextLevelExp` (`KismetMathLibrary.FTrunc` (* _nextlevelexp 1.1)))
        (bind _enumvalue (foreach `/Game/Blueprints/VitalTypes`)
          (:`LoopBody`
            (bind _returnvalue (`KismetMathLibrary.Conv_ByteToInt` _enumvalue))
            (bind (_curval _maxval _buffval _levelmod) (break `/Game/Blueprints/Vital` (`KismetArrayLibrary.Array_Get` _vitals _returnvalue)))
            (bind _returnvalue_2 (`KismetMathLibrary.FTrunc` (* _maxval _levelmod)))
            (`KismetArrayLibrary.Array_Set` _vitals _returnvalue (make `/Game/Blueprints/Vital` _returnvalue_2 _returnvalue_2 _buffval _levelmod))))))))

(fn `LoadStats`
  (bind _asnaga_quest (cast `/Game/Blueprints/NagaQuest` (`GameplayStatics.GetGameMode`)))
  (if (`/Game/Blueprints/NagaQuest.LoadedGame` _asnaga_quest)
    (bind _returnvalue (`GameplayStatics.LoadGameFromSlot` (`KismetSystemLibrary.GetDisplayName` _asnaga_quest)))
    (bind _asnaga_quest_save_game (cast `/Game/Blueprints/NagaQuestSaveGame` _returnvalue))
    (set `self.Vitals` (`/Game/Blueprints/NagaQuestSaveGame.Vitals` _asnaga_quest_save_game))
    (set `self.Exp` (`/Game/Blueprints/NagaQuestSaveGame.Exp` _asnaga_quest_save_game))
    (set `self.NextLevelExp` (`/Game/Blueprints/NagaQuestSaveGame.NextLevelExp` _asnaga_quest_save_game))
    (set `self.Level` (`/Game/Blueprints/NagaQuestSaveGame.Level` _asnaga_quest_save_game))))

(fn `SetupHud`
  (bind _returnvalue (`Controller.CastToPlayerController` (`self.GetController`)))
  (bind _returnvalue_2 (`|CreateWidget` "/Game/Blueprints/StatsUI.StatsUI_C" _returnvalue))
  (`UserWidget.AddToViewport` _returnvalue_2 0))

(fn `SetupVitals`
  (`KismetArrayLibrary.Array_Resize` (`self.Vitals`) (enumcount `/Game/Blueprints/VitalTypes`))
  (bind _enumvalue (foreach `/Game/Blueprints/VitalTypes`)
    (:`LoopBody`
      (`KismetArrayLibrary.Array_Set` (`self.Vitals`) (`KismetMathLibrary.Conv_ByteToInt` (enumliteral `/Game/Blueprints/VitalTypes` _enumvalue)) (make `/Game/Blueprints/Vital` 100)))))

(fn `UserConstructionScript`)